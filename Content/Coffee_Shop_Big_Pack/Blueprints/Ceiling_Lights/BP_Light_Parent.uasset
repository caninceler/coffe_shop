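; Parent Blueprint for coffee shop ceiling lights, pairing a configurable spot light with an emissive fixture mesh.
; The construction script applies optional mesh and plastic material overrides, configures the spot light, and derives emissive color from temperature.
; TurnON, TurnOFF and TurnTOGGLE events update light visibility and emissive strength.
; Emissive strength scales with intensity over source radius, using a larger multiplier at construction than in the events.
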(event Custom|Turn%20ON
  (Variables|Default|SetON true)
  (Rendering|SetVisibility (Variables|Default|GetSpotLight) (Variables|Default|GetON) false)
  (Rendering|Material|SetScalarParameterValueonMaterials (Variables|Default|GetSM_Ceiling_Light) "Emissive" (/ (* (Math|Conversions|ToFloat(Boolean) (Variables|Default|GetON)) (Variables|Default|GetIntensity%20%28cd%29) 1e+01) (Variables|Default|GetSource%20Radius))))

(event Custom|Turn%20OFF
  (Variables|Default|SetON false)
  (Rendering|SetVisibility (Variables|Default|GetSpotLight) (Variables|Default|GetON) false)
  (Rendering|Material|SetScalarParameterValueonMaterials (Variables|Default|GetSM_Ceiling_Light) "Emissive" (/ (* (Math|Conversions|ToFloat(Boolean) (Variables|Default|GetON)) (Variables|Default|GetIntensity%20%28cd%29) 1e+01) (Variables|Default|GetSource%20Radius))))

(event Custom|Turn%20TOGGLE
  (Variables|Default|SetON (not (Variables|Default|GetON)))
  (Rendering|SetVisibility (Variables|Default|GetSpotLight) (Variables|Default|GetON) false)
  (Rendering|Material|SetScalarParameterValueonMaterials (Variables|Default|GetSM_Ceiling_Light) "Emissive" (/ (* (Math|Conversions|ToFloat(Boolean) (Variables|Default|GetON)) (Variables|Default|GetIntensity%20%28cd%29) 1e+01) (Variables|Default|GetSource%20Radius))))

(fn ConstructionScript
  (bind _spotlight (Variables|Default|GetSpotLight))
  (bind _sm_ceiling_light (Variables|Default|GetSM_Ceiling_Light))
  (bind _plastic_material (Variables|Default|GetPlastic%20Material))
  (Utilities|FlowControl|Sequence
    (:then_0
      (Rendering|Material|SetVectorParameterValueonMaterials (Variables|Default|GetSM_Ceiling_Light) "Emissive Color" (Utilities|ColorTemperaturetoRGB (Variables|Default|GetTemperature))))
    (:then_1
      (Utilities|IsValid (Variables|Default|GetMesh)
        (:Is%20Valid
          (Components|StaticMesh|SetStaticMesh (Variables|Default|GetSM_Ceiling_Light) (Variables|Default|GetMesh)))))
    (:then_2
      (Rendering|Material|SetScalarParameterValueonMaterials _sm_ceiling_light "Emissive" (/ (* (Math|Conversions|ToFloat(Boolean) (Variables|Default|GetON)) (Variables|Default|GetIntensity%20%28cd%29) 3e+01) (Variables|Default|GetSource%20Radius)))
      (Utilities|IsValid _plastic_material
        (:Is%20Valid
          (Rendering|Material|SetMaterialbyName _sm_ceiling_light "Plastic" _plastic_material))))
    (:then_3
      (Rendering|Components|Light|SetIntensity _spotlight (Variables|Default|GetIntensity%20%28cd%29))
      (Class|LightComponent|SetTemperature _spotlight (Variables|Default|GetTemperature))
      (Rendering|Lighting|SetInnerConeAngle _spotlight (Variables|Default|GetInner%20Cone%20Angle))
      (Rendering|Lighting|SetOuterConeAngle _spotlight (Variables|Default|GetOuter%20Cone%20Angle))
      (Rendering|SetVisibility _spotlight (Variables|Default|GetON) false)
      (Rendering|Lighting|SetAttenuationRadius _spotlight (Variables|Default|GetAttenuation%20Radius))
      (Class|PointLightComponent|SetSourceRadius _spotlight (Variables|Default|GetSource%20Radius)))))