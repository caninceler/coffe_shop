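; Interactable exterior door for the coffee shop pack that swings open and closed and toggles a widget on box overlap.
; Interact drives a timeline forward or in reverse, with separate open and close curves picked by direction scaling the yaw angle.
; The open sound plays at the start, while the close sound plays when the swing finishes.
; The construction script applies start-open state, material and mesh overrides, an optional sign, and strips interaction components when disabled.
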(event EventInteract
  (if (Variables|Default|GetInteractable)
    (if (not (Audio|Components|Audio|IsPlaying (Variables|Default|GetDoor%20Timeline)))
      (Variables|Default|SetDoor%20Open (not (Variables|Default|GetDoor%20Open)))
      (if (Variables|Default|GetDoor%20Open)
        (Audio|PlaySoundatLocation "/Game/Coffee_Shop_Big_Pack/Sound/Cue/SC_Door_Open.SC_Door_Open" (Transformation|GetActorLocation) "0, 0, 0" 2.0 1.0 0.0 "/Game/Coffee_Shop_Big_Pack/Sound/ATT_Doors.ATT_Doors" 0 0 0)
        (bind (_direction _door_open _door_close) (Timeline|Door%20Timeline Play)
          (:Update
            (Transformation|SetRelativeRotation (Variables|Default|GetDoor) (Math|Rotator|MakeRotator 0.0 0.0 (* (Math|Float|SelectFloat _door_open _door_close (Utilities|Enum|Equal(Enum) _direction "Forward")) (Variables|Default|GetDoor%20Opened%20Angle))) false false))
          (:Finished
            (if (not (Variables|Default|GetDoor%20Open))
              (Audio|PlaySoundatLocation "/Game/Coffee_Shop_Big_Pack/Sound/Wav/S_Door_Close.S_Door_Close" (Transformation|GetActorLocation) "0, 0, 0" 1.0 1.0 0.0 "/Game/Coffee_Shop_Big_Pack/Sound/ATT_Doors.ATT_Doors" 0 0 0))))
        (else
          (Class|AudioMixerBlueprintLibrary|PrimeSoundCueforPlayback "/Game/Coffee_Shop_Big_Pack/Sound/Cue/SC_Door_Close.SC_Door_Close")
          (Timeline|Door%20Timeline Reverse))))))

(event EventOverlap
  (params (End%20Overlap :type Boolean) (Component :type Actor%20Component%20Object%20Reference))
  (bind _widget (Variables|Default|GetWidget))
  (if (Variables|Default|GetInteractable)
    (if (== Component (Variables|Default|GetBox))
      (if End%20Overlap
        (Rendering|SetVisibility _widget false false)
        (else
          (Rendering|SetVisibility _widget true false))))))

(fn ConstructionScript
  (bind _frame_mesh (Variables|Default|GetFrame%20Mesh))
  (bind _sign_mesh (Variables|Default|GetSign%20Mesh))
  (bind _door_mesh (Variables|Default|GetDoor%20Mesh))
  (bind _wall_material (Variables|Default|GetWall%20Material))
  (Utilities|FlowControl|Sequence
    (:then_1
      (if (Variables|Default|GetDoor%20Open)
        (Transformation|SetRelativeRotation (Variables|Default|GetDoor) (Math|Rotator|MakeRotator 0.0 0.0 (Variables|Default|GetDoor%20Opened%20Angle)) false false)
        (Components|Timeline|SetNewTime (Variables|Default|GetDoor%20Timeline) 3.5)))
    (:then_2
      (Utilities|IsValid _wall_material
        (:Is%20Valid
          (Rendering|Material|SetMaterialbyName (Variables|Default|GetDoor_Frame) "Plastic" _wall_material))))
    (:then_4
      (if (not (Variables|Default|GetInteractable))
        (Components|DestroyComponent (Variables|Default|GetBox))))
    (:then_6
      (Utilities|FlowControl|Sequence
        (:then_0
          (Utilities|IsValid _frame_mesh
            (:Is%20Valid
              (Components|StaticMesh|SetStaticMesh (Variables|Default|GetDoor_Frame) _frame_mesh))))
        (:then_1
          (Utilities|IsValid _door_mesh
            (:Is%20Valid
              (Components|StaticMesh|SetStaticMesh (Variables|Default|GetDoor) _door_mesh)
              (if (not (== _door_mesh "/Game/Coffee_Shop_Big_Pack/Meshes/Doors/SM_Door_Nanite.SM_Door_Nanite"))
                (Components|DestroyComponent (Variables|Default|GetSM_Door_Glass))))))))
    (:then_7
      ;[1 1 1] Sign Mesh
      (if (Variables|Default|GetSign)
        (bind _returnvalue (AddComponent|AddStaticMeshComponent false))
        (Transformation|AttachComponentToComponent _returnvalue (Variables|Default|GetDoor) "Sign" "KeepRelative" "KeepRelative" "KeepRelative" true)
        (Utilities|IsValid _sign_mesh
          (:Is%20Valid
            (Components|StaticMesh|SetStaticMesh _returnvalue _sign_mesh)))))))